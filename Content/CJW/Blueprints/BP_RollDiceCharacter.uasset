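; BP_RollDiceCharacter is a character Blueprint that sets up a dice-roll scene when play begins.
; It adds the ThrowDIceUi widget to the viewport and restricts its SceneCaptureComponent2D to showing only its own Mesh.
; After a fixed delay, it detaches HandComp, then finds the BP_Dice actor and nudges it upward along its local Z axis.
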(event `self.ReceiveBeginPlay`
  (bind _returnvalue (`|CreateWidget` "/Game/CJW/UI/ThrowDIceUi.ThrowDIceUi_C"))
  (`UserWidget.AddToViewport` _returnvalue 0)
  (`SceneCaptureComponent.ShowOnlyComponent` (`self.SceneCaptureComponent2D`) (`self.Mesh`))
  (`KismetSystemLibrary.Delay` 4.0)
  (`SceneComponent.K2_DetachFromComponent` (`self.handComp`) "KeepRelative" "KeepRelative" "KeepRelative" true)
  (bind _returnvalue_2 (`GameplayStatics.GetActorOfClass` "/Game/CJW/Blueprints/BP_Dice.BP_Dice_C"))
  (bind _asbp_dice (cast `/Game/CJW/Blueprints/BP_Dice` _returnvalue_2))
  (`self.K2_AddActorLocalOffset` _asbp_dice (0.0 0.0 40.0) false false))

(fn `UserConstructionScript`)
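; BP_PartyPlayer is a board-game party player that rolls a die and walks along linked spaces.
; RollDice blends the camera to the player, picks a random step count and starts MoveToSpace.
; MoveToSpace uses AI movement along each space's first NextSpace link, recursing until steps run out.
; TurnEnded then prints a coin gain or loss placeholder for blue or red spaces and calls OnTurnEnded.
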(event `self.ReceiveBeginPlay`)

(event `MoveToSpace`
  (params (CurrentSpace :type "/Game/CJW/Blueprints/BP_BlueBoardSpace Object Reference"))
  (bind _output (`|GetArrayItem` (`/Game/CJW/Blueprints/BP_BlueBoardSpace.NextSpace` CurrentSpace)))
  ;[1 1 1] 나온 주사위의 수만큼 이동하는 노드 , 이동하고 주사위의 수가 남아있다면 다음 장소를 얻어와서 주사위 수가 0이 될때까지 반복한다
  (set `self.CurrentSpace` _output)
  (`|AIMoveTo` self (0.0 0.0 0.0) _output
    (:`OnSuccess`
      (bind _result (`/Engine/EditorBlueprintResources/StandardMacros.DecrementInt` (`self.MoveRemaining`))
        (:`  `
          (`KismetSystemLibrary.PrintString` (`KismetStringLibrary.Conv_IntToString` (`self.MoveRemaining`)))
          (if (> _result 0)
            (`self.MoveToSpace` (`self.CurrentSpace`))
            (else
              (`self.TurnEnded`))))))))

(event `TurnEnded`
  ;[1 1 1] 이동이 완료되면 , 해당 발판 상호작용 시작하기
  (`|ExecutionSequence`
    (:`then_0`
      (switch `/Game/CJW/Enum/SpaceState` (`/Game/CJW/Blueprints/BP_BlueBoardSpace.SpaceState` (`self.CurrentSpace`))
        (:`NewEnumerator0`
          ;[1 0.03478 0.5022] 각 발판 당 특성에 해당하는  함수 호출
          (`KismetSystemLibrary.PrintString` "+3coins"))
        (:`NewEnumerator1`
          (`KismetSystemLibrary.PrintString` "-3coin"))))
    (:`then_1`
      ;[1 1 1] 턴이 끝났다는 신호 보내기
      (`self.OnTurnEnded`))))

(event `RollDice`
  ;[1 1 1] 카메라 가져오기
  (`PlayerController.SetViewTargetWithBlend` (`GameplayStatics.GetPlayerController` 0) self 1.0 "VTBlend_Linear" 0.0 false)
  ;[1 1 1] 주사위를 던져서 몇칸갈지 정하기
  (set `self.MoveRemaining` (`KismetMathLibrary.RandomIntegerInRange` 1 6))
  (`self.MoveToSpace` (`self.CurrentSpace`)))

(fn `UserConstructionScript`)
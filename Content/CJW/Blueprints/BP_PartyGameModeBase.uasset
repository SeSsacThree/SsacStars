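; BP_PartyGameModeBase is a party game mode sketching round and turn flow, but its events are empty and that logic is disconnected.
; The unwired chains copy all BP_PartyPlayer actors from TurnOrder into RoundOrder, binding each current player's OnTurnEnded to NextTurn.
; They pop finished players until the list empties, then decrement Round and restart after a delay.
; CreateWidget adds MainUi to the viewport, though its only call is also unwired.
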(event `ThrowDiceShot`)

(event `CreateWidget`
  (bind _returnvalue (`|CreateWidget` "/Game/CJW/UI/MainUi.MainUi_C"))
  (`UserWidget.AddToViewport` _returnvalue 0))

(event `self.ReceiveBeginPlay`)

(event `InitialRound`
  ;[1 1 1] 라운드 시작-해당 라운드의 플레이어의 정보를 넣고 그 플레이어의 라운드를 시작시킨다
)

(event `StartTurn`
  ;[1 1 1] 첫번째 플레이어 턴시작
)

(event `NextTurn`
  ;[1 1 1] 그다음 플레이어 턴 시작
)

(event `EndRound`)

(fn `UserConstructionScript`)